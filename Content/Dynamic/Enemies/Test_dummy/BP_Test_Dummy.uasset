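; Test dummy enemy that attacks the player, suffers weapon status effects and drops cores.
; Attack halts movement, plays a zombie montage and uses a sphere overlap to deal damage.
; Tick applies the player's weapon effect while StatBuildUp is full, without resetting it, and at exactly zero HP destroys the actor and randomly credits a core to the player.
; A Range overlap toggles the health bar.
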(event `Attack`
  (if (not (`self.Is Attacking?`))
    (set `self.Is Attacking?` true)
    (`CharacterMovementComponent.DisableMovement` (`self.CharacterMovement`))
    (`|PlayMontage` (`self.Mesh`) "/Game/Static/BSP_ZombieAnims/Animations/Standing/Attack/AM_ZombieAttack.AM_ZombieAttack"
      (:`then`
        (bind _outactors (`KismetSystemLibrary.SphereOverlapActors` (`SceneComponent.K2_GetComponentLocation` (`self.Sphere attack`)) 100.0 (`|MakeArray` "ObjectTypeQuery3" :!type "EObjectTypeQuery Enum") "/Game/Dynamic/ThirdPerson/Player_Blueprints/BP_ThirdPersonCharacter.BP_ThirdPersonCharacter_C" (`|MakeArray` self :!type "Actor Object Reference")))
        (if (`KismetArrayLibrary.Array_IsValidIndex` _outactors)
          (bind _asbp_third_person_character (cast `/Game/Dynamic/ThirdPerson/Player_Blueprints/BP_ThirdPersonCharacter` (`GameplayStatics.GetPlayerCharacter` 0)))
          (set `/Game/Dynamic/ThirdPerson/Player_Blueprints/BP_ThirdPersonCharacter.Current HP` (- (`/Game/Dynamic/ThirdPerson/Player_Blueprints/BP_ThirdPersonCharacter.Current HP` _asbp_third_person_character) 10.0) _asbp_third_person_character)
          (`KismetSystemLibrary.Delay` 3.0)
          (set `self.Is Attacking?` false)))
      (:`OnCompleted`
        (`KismetSystemLibrary.Delay` 1.0)
        (`CharacterMovementComponent.SetMovementMode` (`self.CharacterMovement`) "MOVE_Walking" 0)))))

(event `self.ReceiveTick`
  (params (DeltaSeconds :type "Float (single-precision)"))
  (`|ExecutionSequence`
    (:`then_0`
      (if (== (`self.HP`) 0.0)
        (`self.K2_DestroyActor`)
        (`self.Item drop`)))
    (:`then_1`
      (if (>= (`self.Stat Build Up`) 100.0)
        (`self.Effect build up`)))))

(event `self.Range.OnComponentBeginOverlap`
  (params (OverlappedComponent :type "PrimitiveComponent Object Reference") (OtherActor :type "Actor Object Reference") (OtherComp :type "PrimitiveComponent Object Reference") (OtherBodyIndex :type Integer) (bFromSweep :type Boolean) (SweepResult :type "HitResult Structure (by ref)"))
  (`SceneComponent.SetVisibility` (`self.Health Bar`) true false))

(event `self.Range.OnComponentEndOverlap`
  (params (OverlappedComponent :type "PrimitiveComponent Object Reference") (OtherActor :type "Actor Object Reference") (OtherComp :type "PrimitiveComponent Object Reference") (OtherBodyIndex :type Integer))
  (`SceneComponent.SetVisibility` (`self.Health Bar`) false false))

(fn `Effect build up`
  (bind _asbp_third_person_character (cast `/Game/Dynamic/ThirdPerson/Player_Blueprints/BP_ThirdPersonCharacter` (`GameplayStatics.GetPlayerCharacter` 0)))
  (switch `string` (`/Game/Dynamic/ThirdPerson/Player_Blueprints/BP_ThirdPersonCharacter.Weapon Stat 1` _asbp_third_person_character)
    (:`Frost`
      (`KismetSystemLibrary.PrintString` "frost")
      (set `self.HP` (- (`self.HP`) 30.0)))
    (:`Bleed`
      (`KismetSystemLibrary.PrintString` "Bleed")
      (set `self.HP` (- (`self.HP`) 20.0)))
    (:`Fire`
      (`KismetSystemLibrary.PrintString` "frost")
      (set `self.HP` (- (`self.HP`) 10.0)))
    (:`Lifesteal`
      (`KismetSystemLibrary.PrintString` "frost")
      (set `self.HP` (- (`self.HP`) 20.0))
      (set `/Game/Dynamic/ThirdPerson/Player_Blueprints/BP_ThirdPersonCharacter.Current HP` (+ (`/Game/Dynamic/ThirdPerson/Player_Blueprints/BP_ThirdPersonCharacter.Current HP` _asbp_third_person_character) 20.0) _asbp_third_person_character))
    (:`Scarlet Rot`
      (`KismetSystemLibrary.PrintString` "frost")
      (set `self.HP` (- (`self.HP`) 1.0)))))

(fn `Item drop`
  (switch `int` (`KismetMathLibrary.RandomIntegerInRange` 0 6)
    (:`2`
      (`KismetSystemLibrary.PrintString` "basic core" :!label _label)
      (bind _asbp_third_person_character (cast `/Game/Dynamic/ThirdPerson/Player_Blueprints/BP_ThirdPersonCharacter` (`GameplayStatics.GetPlayerCharacter` 0)))
      (set `/Game/Dynamic/ThirdPerson/Player_Blueprints/BP_ThirdPersonCharacter.BasicCoreNum` (+ (`/Game/Dynamic/ThirdPerson/Player_Blueprints/BP_ThirdPersonCharacter.BasicCoreNum` _asbp_third_person_character) 1) _asbp_third_person_character))
    (:`3`
      (goto _label))
    (:`4`
      (`KismetSystemLibrary.PrintString` "power core" :!label _label_2)
      (bind _asbp_third_person_character_2 (cast `/Game/Dynamic/ThirdPerson/Player_Blueprints/BP_ThirdPersonCharacter` (`GameplayStatics.GetPlayerCharacter` 0)))
      (set `/Game/Dynamic/ThirdPerson/Player_Blueprints/BP_ThirdPersonCharacter.HighCoreNum` (+ (`/Game/Dynamic/ThirdPerson/Player_Blueprints/BP_ThirdPersonCharacter.HighCoreNum` _asbp_third_person_character_2) 1) _asbp_third_person_character_2))
    (:`5`
      (goto _label_2))
    (:`6`
      (`KismetSystemLibrary.PrintString` "super core")
      (bind _asbp_third_person_character_3 (cast `/Game/Dynamic/ThirdPerson/Player_Blueprints/BP_ThirdPersonCharacter` (`GameplayStatics.GetPlayerCharacter` 0)))
      (set `/Game/Dynamic/ThirdPerson/Player_Blueprints/BP_ThirdPersonCharacter.SuperCoreNum` (+ (`/Game/Dynamic/ThirdPerson/Player_Blueprints/BP_ThirdPersonCharacter.SuperCoreNum` _asbp_third_person_character_3) 1) _asbp_third_person_character_3))))

(fn `UserConstructionScript`)